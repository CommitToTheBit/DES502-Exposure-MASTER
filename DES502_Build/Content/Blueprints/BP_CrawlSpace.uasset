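; BP_CrawlSpace is a spline-based crawl path that links to nearby crawl spaces through left/right forks.
; On entry, it finds spaces starting near its end, picks the nearest per side and spawns temporary two-point transition splines matching endpoint tangents and up vectors.
; ChooseFork sets NextCrawlSpace near the end, favouring preferred, then previous fork.
; On exit, transitions destroy themselves and normal spaces destroy unchosen forks; forking only works forward.
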(event Custom|OnEntered
  ;[0.05098 0.05098 0.05098] ON ENTERED: Construct temporary 'transition' crawl spaces...
  (if (not (Variables|Default|GetForkTransition))
    (CallFunction|ConstructFork true)))

(event Custom|OnExited
  ;[0.05098 0.05098 0.05098] ON EXITED: Destroy transition crawl spaces, where possible...
  (if (Variables|Default|GetForkTransition)
    (Actor|DestroyActor)
    (else
      (bind _keys (Utilities|Map|Keys (Variables|Default|GetForkForward)))
      (for _array_element _keys
        (if (not (== (Variables|Default|GetNextCrawlSpace) (.Value (Utilities|Map|Find (Variables|Default|GetForkForward) _array_element))))
          (Actor|DestroyActor (.Value (Utilities|Map|Find (Variables|Default|GetForkForward) _array_element)))))
      (bind _keys_2 (Utilities|Map|Keys (Variables|Default|GetForkBackward)))
      (for _array_element_2 _keys_2
        (if (not (== (Variables|Default|GetNextCrawlSpace) (.Value (Utilities|Map|Find (Variables|Default|GetForkBackward) _array_element_2))))
          (Actor|DestroyActor (.Value (Utilities|Map|Find (Variables|Default|GetForkBackward) _array_element_2))))))))

(fn ConstructionScript)

(fn ConstructFork
  (params (Forward :type Boolean))
  (bind _spline (Variables|Default|GetSpline))
  ;[0.2159 0.05127 0.05127] // FIXME: CONSTRUCT FORK: Only supported in one direction...
  (if Forward
    ;[0.05098 0.05098 0.05098] ...For each crawl space that can be forked to, create a temporary 'transition' crawl space in between...
    (bind _nearestcrawlspaces (CallFunction|GetNearbyCrawlSpaces true))
    (bind _forkedcrawlspaces (CallFunction|GetForkedCrawlSpaces _nearestcrawlspaces Forward))
    (if Forward
      (Utilities|Map|Clear (Variables|Default|GetForkForward))
      (bind _keys (Utilities|Map|Keys _forkedcrawlspaces))
      (for _array_element _keys
        (bind _returnvalue (Game|SpawnActorfromClass "BP_CrawlSpace_C" (Spline|GetTransformatDistanceAlongSpline _spline (Spline|GetSplineLength _spline) "Local" false) "Undefined" 0 0))
        (Utilities|IsValid (.Value (Utilities|Map|Find _forkedcrawlspaces _array_element))
          (:Is%20Valid
            (CallFunction|ConstructTransition _returnvalue self (.Value (Utilities|Map|Find _forkedcrawlspaces _array_element)) true)
            (Utilities|Map|Add (Variables|Default|GetForkForward) _array_element _returnvalue)
            (if (== (Utilities|Map|Length (Variables|Default|GetForkForward)) 1)
              (Variables|Default|SetNextCrawlSpace _returnvalue))))))))

(fn ConstructTransition
  (params (FromCrawlSpace :type BP%20Crawl%20Space%20Object%20Reference) (ToCrawlSpace :type BP%20Crawl%20Space%20Object%20Reference) (Forward :type Boolean))
  ;[0.05098 0.05098 0.05098] CONSTRUCT TRANSITION: Make direction considerations... // NB: Ignores possibility of changing direction across forks!
  (LocalVariables|SetFromSpline (Variables|BP_CrawlSpace_C|GetSpline FromCrawlSpace))
  (LocalVariables|SetToSpline (Variables|BP_CrawlSpace_C|GetSpline ToCrawlSpace))
  (if Forward
    (LocalVariables|SetFromCrawlDistance (Spline|GetSplineLength (LocalVariables|GetFromSpline)))
    (LocalVariables|SetToCrawlDistance 0.0)
    (else
      (LocalVariables|SetFromCrawlDistance 0.0)
      (LocalVariables|SetToCrawlDistance (Spline|GetSplineLength (LocalVariables|GetToSpline)))))
  ;[0.05098 0.05098 0.05098] ...Construct a spline from exactly two points... // FIXME: How does this transition become smoother?
  (Variables|Default|SetForkTransition true)
  (Spline|ClearSplinePoints (Variables|Default|GetSpline) true)
  (Spline|AddSplinePoint (Variables|Default|GetSpline) (Spline|GetLocationatDistanceAlongSpline (LocalVariables|GetFromSpline) (LocalVariables|GetFromCrawlDistance) "World") "World" true)
  (Class|SplineComponent|SetUpVectoratSplinePoint (Variables|Default|GetSpline) 0 (Class|SplineComponent|GetUpVectoratDistanceAlongSpline (LocalVariables|GetFromSpline) (LocalVariables|GetFromCrawlDistance) "World") "World" true)
  (Spline|SetTangentatSplinePoint (Variables|Default|GetSpline) 0 (Spline|GetTangentatDistanceAlongSpline (LocalVariables|GetFromSpline) (LocalVariables|GetFromCrawlDistance) "World") "World" true)
  (Spline|AddSplinePoint (Variables|Default|GetSpline) (Spline|GetLocationatDistanceAlongSpline (LocalVariables|GetToSpline) (LocalVariables|GetToCrawlDistance) "World") "World" true)
  (Class|SplineComponent|SetUpVectoratSplinePoint (Variables|Default|GetSpline) 1 (Class|SplineComponent|GetUpVectoratDistanceAlongSpline (LocalVariables|GetToSpline) (LocalVariables|GetToCrawlDistance) "World") "World" true)
  (Spline|SetTangentatSplinePoint (Variables|Default|GetSpline) 1 (Spline|GetTangentatDistanceAlongSpline (LocalVariables|GetToSpline) (LocalVariables|GetToCrawlDistance) "World") "World" true)
  (Variables|Default|SetNextCrawlSpace ToCrawlSpace))

(fn GetNearbyCrawlSpaces
  (params (Forward :type Boolean))
  (bind _spline (Variables|Default|GetSpline))
  (bind _returnvalue (Spline|GetSplineLength _spline))
  (bind _returnvalue_2 (Spline|GetLocationatDistanceAlongSpline _spline _returnvalue "World"))
  ;[0.2159 0.05127 0.05127] // FIXME: GET NEARBY CRAWLSPACES: Only supported in one direction...
  (if Forward
    ;[0.05098 0.05098 0.05098] ...Return all nearby crawl spaces than we can fork to, nearest first...
    (bind _outactors (Actor|GetAllActorsOfClass "BP_CrawlSpace_C"))
    (for _array_element _outactors
      (if (not (or (or (Variables|BP_CrawlSpace_C|GetIgnoreAtFork _array_element) (Variables|BP_CrawlSpace_C|GetForkTransition _array_element)) (== _array_element self)))
        (bind (_array_element_2 _array_index) (Utilities|Array|ForEachLoopwithBreak (LocalVariables|GetCrawlSpaces) :!label _label)
          (:LoopBody
            (if (< (Math|Vector|VectorLength (- (Spline|GetLocationatDistanceAlongSpline (Variables|BP_CrawlSpace_C|GetSpline _array_element) 0.0 "World") _returnvalue_2)) (Math|Vector|VectorLength (- (Spline|GetLocationatDistanceAlongSpline (Variables|BP_CrawlSpace_C|GetSpline _array_element_2) 0.0 "World") _returnvalue_2)))
              (Utilities|Array|Insert (LocalVariables|GetCrawlSpaces) _array_element _array_index)
              (goto _label Break)))
          (:Completed
            (if (and (not (Utilities|Array|ContainsItem (LocalVariables|GetCrawlSpaces) _array_element)) (< (Math|Vector|VectorLength (- (Spline|GetLocationatDistanceAlongSpline (Variables|BP_CrawlSpace_C|GetSpline _array_element) 0.0 "World") _returnvalue_2)) 1e+02))
              (Utilities|Array|Add (LocalVariables|GetCrawlSpaces) _array_element))))))
    (return (LocalVariables|GetCrawlSpaces))
    (else
      (return 0))))

(fn GetForkedCrawlSpaces
  (params (NearbyCrawlSpaces :type Array%20of%20BP%20Crawl%20Space%20Object%20References) (Forward :type Boolean))
  (bind _spline (Variables|Default|GetSpline))
  (bind _crawlspaces (LocalVariables|GetCrawlSpaces))
  (bind _crawlspaces_2 (LocalVariables|GetCrawlSpaces))
  (bind _returnvalue (Spline|GetSplineLength _spline))
  (bind _returnvalue_2 (Spline|GetTangentatDistanceAlongSpline _spline _returnvalue "World"))
  ;[0.2159 0.05127 0.05127] // FIXME: GET FORKED CRAWL SPACES: Only supported in one direction...
  (if Forward
    ;[0.05098 0.05098 0.05098] ...Of the nearby crawl spaces, find the nearest 'forward and to the left/right' of our own endpoint... // NB: Could trivially extend this to a maximum of four, 'WASD' forks...
    (bind _array_element (Utilities|Array|ForEachLoopwithBreak NearbyCrawlSpaces :!label _label)
      (:LoopBody
        (if (>= (Utilities|Map|Length (LocalVariables|GetCrawlSpaces)) 2)
          (goto _label Break)
          (elif (<= (Class|KismetMathLibrary|DegAcos (Math|Vector|DotProduct (Math|Vector|Normalize (- (Spline|GetLocationatDistanceAlongSpline (Variables|BP_CrawlSpace_C|GetSpline _array_element) 0.0 "World") (Spline|GetLocationatDistanceAlongSpline _spline _returnvalue "World"))) (Math|Vector|Normalize _returnvalue_2))) 1.8e+02)
            (if (> (Math|Vector|DotProduct (Math|Vector|Normalize (- (Spline|GetLocationatDistanceAlongSpline (Variables|BP_CrawlSpace_C|GetSpline _array_element) 0.0 "World") (Spline|GetLocationatDistanceAlongSpline _spline _returnvalue "World"))) (Math|Vector|CrossProduct _returnvalue_2 (Class|SplineComponent|GetUpVectoratDistanceAlongSpline _spline _returnvalue "World"))) 0.0)
              (if (not (Utilities|Map|Contains _crawlspaces_2 "Left"))
                (Utilities|Map|Add _crawlspaces_2 "Left" _array_element))
              (elif (not (Utilities|Map|Contains _crawlspaces "Right"))
                (Utilities|Map|Add _crawlspaces "Right" _array_element))))))
      (:Completed
        (return (LocalVariables|GetCrawlSpaces))))))

(fn ChooseFork
  (params (PreviousFork :type String) (PreferredFork :type String) (Forward :type Boolean) (DistanceFromFork :type Float%20%28double-precision%29))
  (bind _forkforward (Variables|Default|GetForkForward))
  (bind _forkforward_2 (Variables|Default|GetForkForward))
  (bind _forkforward_3 (Variables|Default|GetForkForward))
  (bind (_value _returnvalue) (Utilities|Map|Find _forkforward_2 PreviousFork))
  (bind (_value_2 _returnvalue_2) (Utilities|Map|Find _forkforward_3 PreferredFork))
  ;[0.2159 0.05127 0.05127] // FIXME: CAN CHOOSE FORK: Only supported in one direction...
  (if Forward
    ;[0.05098 0.05098 0.05098] ...Check if we have permission to do anything...
    (if (> DistanceFromFork (- (Spline|GetSplineLength (Variables|Default|GetSpline)) (* 5.0 (Variables|Default|GetCrawlStepSize))))
      ;[0.05098 0.05098 0.05098] ...Check if the preferred fork is viable...
      (if _returnvalue_2
        (Variables|Default|SetNextCrawlSpace _value_2)
        (return PreferredFork)
        (else
          ;[0.05098 0.05098 0.05098] ...Check if the previous fork is viable...
          (if _returnvalue
            (Variables|Default|SetNextCrawlSpace _value)
            (return PreviousFork)
            (else
              ;[0.05098 0.05098 0.05098] ...Check what choice there actually is...
              (if (> (Utilities|Map|Length (Variables|Default|GetForkForward)) 0)
                (bind _keys (Utilities|Map|Keys _forkforward))
                (Variables|Default|SetNextCrawlSpace (.Value (Utilities|Map|Find _forkforward (Utilities|Array|Get(acopy) _keys)))))
              (if (> (Utilities|Map|Length (Variables|Default|GetForkForward)) 1)
                (bind _keys_2 (Utilities|Map|Keys (Variables|Default|GetForkForward)))
                (return (Utilities|Array|Get(acopy) _keys_2))
                (else
                  (return "N/A")))))))
      (else
        (return PreviousFork)))))