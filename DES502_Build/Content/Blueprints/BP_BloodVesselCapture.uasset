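; Blood vessel capture actor that builds a danger-driven ring of procedural vessels for a screen vignette effect.
; BeginPlay spawns seeded BP_BloodVessel actors and arranges them on an ellipse scaled to a hardcoded 16:9 aspect, rotated around the ring.
; While the player moves or Danger changes, Tick updates each vessel with the Danger delta and writes Intensity to the vignette shader's Material Parameter Collection.
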(event EventBeginPlay
  (bind _returnvalue (Transformation|GetActorTransform))
  (bind _returnvalue_2 (/ 1.92e+03 1.08e+03))
  (bind _bloodvesselcount (Variables|Default|GetBloodVesselCount))
  ;[0.05098 0.05098 0.05098] BEGIN PLAY: ...Create reference to BP_FirstPersonCharacter...
  (bind _asbp_first_person_character (Utilities|Casting|CastToBP_FirstPersonCharacter (Game|GetPlayerCharacter 0)))
  (Variables|Default|SetFirstPersonCharacter _asbp_first_person_character)
  (for _index (range 0 (- _bloodvesselcount 1))
    (bind _returnvalue_3 (Game|SpawnActorfromClass "/Game/Blueprints/BP_BloodVessel.BP_BloodVessel_C" _returnvalue "Undefined" 0 0))
    (Utilities|Array|Add (Variables|Default|GetBloodVessels) _returnvalue_3)
    (Class|DESLBloodVessel|Initialize _returnvalue_3 (Variables|/Game/Blueprints/BP_BloodVessel.BP_BloodVessel_C|GetProceduralMesh _returnvalue_3) 0.167 16 (Math|Conversions|ToFloat(Integer) _index))
    (Transformation|SetWorldTransform (Variables|/Game/Blueprints/BP_BloodVessel.BP_BloodVessel_C|GetDefaultSceneRoot _returnvalue_3) (Math|Transform|ComposeTransforms (Math|Transform|MakeTransform (* (* (Math|Float|Sqrt (+ 1.0 (Math|Float|Square _returnvalue_2))) 0.55) (Math|Vector|MakeVector 0.0 (* _returnvalue_2 (Math|Trig|Cos(Radians) (* _index (/ (Math|Float|MultiplybyPi 2.0) _bloodvesselcount)))) (Math|Trig|Sin(Radians) (* _index (/ (Math|Float|MultiplybyPi 2.0) _bloodvesselcount))))) (Math|Rotator|MakeRotator (+ (* (Class|KismetMathLibrary|DegAtan2 (Math|Trig|Sin(Radians) (* _index (/ (Math|Float|MultiplybyPi 2.0) _bloodvesselcount))) (* _returnvalue_2 (Math|Trig|Cos(Radians) (* _index (/ (Math|Float|MultiplybyPi 2.0) _bloodvesselcount))))) -1.0) -9e+01) 0.0 0.0) "1.000000,1.000000,1.000000") (Math|Transform|ComposeTransforms (Math|Transform|MakeTransform "0.500000,0.000000,0.000000" (Math|Rotator|MakeRotator 0.0 0.0 0.0) "1.000000,1.000000,1.000000") _returnvalue)) false false)))

(event EventTick
  (params (DeltaSeconds :type Float%20%28single-precision%29))
  (bind _firstpersoncharacter (Variables|Default|GetFirstPersonCharacter))
  (if (or (!= (Math|Vector|VectorLength (Variables|/Script/Engine.MovementComponent|GetVelocity (Variables|/Script/Engine.Character|GetCharacterMovement _firstpersoncharacter))) 0.0) (!= (- (Variables|/Game/Blueprints/BP_FirstPersonCharacter.BP_FirstPersonCharacter_C|GetDanger _firstpersoncharacter) (Variables|Default|GetIntensity)) 0.0))
    (for _array_element (Variables|Default|GetBloodVessels)
      (Class|DESLSystem|Update _array_element DeltaSeconds (- (Variables|/Game/Blueprints/BP_FirstPersonCharacter.BP_FirstPersonCharacter_C|GetDanger _firstpersoncharacter) (Variables|Default|GetIntensity))))
    (bind _output_get (Variables|Default|SetIntensity (Variables|/Game/Blueprints/BP_FirstPersonCharacter.BP_FirstPersonCharacter_C|GetDanger (Variables|Default|GetFirstPersonCharacter))))
    (Rendering|Material|SetScalarParameterValue "/Game/VFX/VignetteScreenShader_LocalParameters.VignetteScreenShader_LocalParameters" "Intensity" _output_get :!class /Script/Engine.KismetMaterialLibrary)))

(fn ConstructionScript)

(fn GetBloodVesselAngles
  (params (Index :type Integer))
  (bind _output_get (LocalVariables|SetFraction (/ (+ Index 0.5) (Variables|Default|GetBloodVesselCount))))
  (return (* 3.6e+02 _output_get) 0.0))

(fn TickIntensity
  (params (DeltaTime :type Float%20%28double-precision%29) (NewIntensity :type Float%20%28double-precision%29))
  (if (!= NewIntensity (Variables|Default|GetIntensity))
    (Rendering|Material|SetScalarParameterValue "/Game/VFX/VignetteScreenShader_LocalParameters.VignetteScreenShader_LocalParameters" "Intensity" 0.0 :!class /Script/Engine.KismetMaterialLibrary)))