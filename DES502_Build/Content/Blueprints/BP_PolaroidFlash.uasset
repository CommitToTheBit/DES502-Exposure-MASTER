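; BP_PolaroidFlash is a prototype short-lived actor that takes a polaroid picture with a flash the moment it spawns.
; On BeginPlay, once the game instance casts to DESGameInstance, it triggers CaptureScene on its SceneCaptureComponent2D, then a timeline drives the Flash intensity to fade out and destroys the actor.
; Render target assignment, from a debug journal entry or newly created, is disconnected, and saving multiple images remains a FIXME.
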(event EventBeginPlay
  ;[0.2159 0.05127 0.05127] Instantly take picture on spawn... // FIXME: This feels like a prototype, just attach this flash functionality to the eventual full polaroid camera blueprint?
  (bind _asdesgame_instance (Utilities|Casting|CastToDESGameInstance (Game|GetGameInstance)))
  (Rendering|SceneCapture|CaptureScene (Variables|Default|GetSceneCaptureComponent2D) :!class /Script/Engine.SceneCaptureComponent2D)
  ;[0.05098 0.05098 0.05098] ...Then fade the flash out...
  (bind _flashintensity (Timeline|FlashTimeline Play)
    (:Update
      (Rendering|Components|Light|SetIntensity (Variables|Default|GetFlash) _flashintensity))
    (:Finished
      (Actor|DestroyActor))))

(fn ConstructionScript)