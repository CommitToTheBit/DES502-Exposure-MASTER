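; Polaroid camera that is collected on overlap when not player-owned and photographs nearby curios to fill journal entries.
; Shooting runs an ammo check (cost currently zero), then timelines drive the flash and capture while the camera is locked.
; Capture counts recently rendered curios inside the view cone per ID.
; The top-scoring inactive journal entry is activated, logged in the chronology and receives the scene capture in its render target.
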(event OnComponentBeginOverlap(CollisionSphere)
  (params (OverlappedComponent :type Primitive%20Component%20Object%20Reference) (OtherActor :type Actor%20Object%20Reference) (OtherComp :type Primitive%20Component%20Object%20Reference) (OtherBodyIndex :type Integer) (bFromSweep :type Boolean) (SweepResult :type Hit%20Result%20Structure%20%28by%20ref%29))
  (bind _des_gameinstance (Variables|Default|GetDES_GameInstance))
  (bind _gamedata (Variables|/Script/DES502_Build.DESGameInstance|GetGameData _des_gameinstance))
  ;[0.05127 0.05127 0.05127] BEGIN OVERLAP: If not owned by the player, add to counter and destroy...
  (Utilities|Casting|CastToBP_FirstPersonCharacter (Components|GetOwner)
    (:CastFailed
      (Variables|/Script/DES502_Build.DESSaveGame|SetPolaroidInventoried _gamedata (+ (Variables|/Script/DES502_Build.DESSaveGame|GetPolaroidInventoried _gamedata) 1))
      (Actor|DestroyActor))))

(event Input|EnhancedActionEvents|EnhancedInputActionIA_Shoot
  (params (ActionValue :type Boolean) (ElapsedSeconds :type Float%20%28double-precision%29) (TriggeredSeconds :type Float%20%28double-precision%29) (InputAction :type Input%20Action%20Object%20Reference :default "/Game/Prefabs/FirstPerson/Input/Actions/IA_Shoot.IA_Shoot"))
  (bind _flash (Variables|Default|GetFlash))
  ;[0.05 0.05 0.05] IA_SHOOT: If possible, spend polaroid ammo...
  (:Triggered
    (if (== (Variables|/Script/Engine.LightComponentBase|GetIntensity (Variables|Default|GetFlash)) 0.0)
      (bind _fired (CallFunction|ExpendPolaroidAmmo 0))
      (if _fired
        ;[0.05098 0.05098 0.05098] ...Allow animation cancelling...
        (Utilities|FlowControl|Delay 0.15)
        ;[0.117 0.05127 0.117] ...Force player to wait for flash... // FIXME: Add SFX, lighting here...
        (Variables|Default|SetPolaroidLocked true)
        (Utilities|FlowControl|Delay 0.25)
        ;[0.05098 0.05098 0.05098] ...Capture image, with flash... // FIXME: CapturePolaroid does nothing...
        (bind _flash_2 (Timeline|CaptureTimeline SetNewTime)
          (:Update
            (Rendering|Components|Light|SetIntensity (Variables|Default|GetFlash) _flash_2)
            (CallFunction|CapturePolaroid)
            ;[0.05098 0.05098 0.05098] ...Fade the flash out...
            (bind _flash_3 (Timeline|FlashTimeline PlayFromStart)
              (:Update
                (Rendering|Components|Light|SetIntensity _flash _flash_3))
              (:Finished
                (Rendering|Components|Light|SetIntensity _flash 0.0)
                (Variables|Default|SetPolaroidLocked false)
                (Variables|/Script/DES502_Build.DESGameInstance|SetPolaroidPressed (Variables|Default|GetDES_GameInstance) false)
                ;[0.05098 0.05098 0.05098] BUGFIX: If the iron sights have been released since the camera animation started, then lower them...
                (if (not (Input|EnhancedActionValues|GetIA_Zoomed))
                  (Default|DelayedIAZoomOut (Variables|Default|GetFirstPersonCharacter)))))))))))

(fn ConstructionScript
  (|CallParentFunction))

(fn ExpendPolaroidAmmo
  (params (Cost :type Integer))
  (bind _des_gameinstance (Variables|Default|GetDES_GameInstance))
  (bind _gamedata (Variables|/Script/DES502_Build.DESGameInstance|GetGameData _des_gameinstance))
  ;[0.05098 0.05098 0.05098] EXPEND POLAROID AMMO: Check if polaroid will be fired...
  (bind _output_get (Variables|/Script/DES502_Build.DESGameInstance|SetPolaroidPressed (Variables|Default|GetDES_GameInstance) (<= Cost (Variables|/Script/DES502_Build.DESSaveGame|GetPolaroidAmmo _gamedata))))
  (if _output_get
    (Variables|/Script/DES502_Build.DESSaveGame|SetPolaroidAmmo _gamedata (- (Variables|/Script/DES502_Build.DESSaveGame|GetPolaroidAmmo _gamedata) Cost)))
  (return _output_get))

(fn CapturePolaroid
  (bind _scenecapturecomponent2d (Variables|Default|GetSceneCaptureComponent2D))
  (bind _des_gameinstance (Variables|Default|GetDES_GameInstance))
  (bind _journalmanager (Variables|/Script/DES502_Build.DESGameInstance|GetJournalManager _des_gameinstance))
  (bind _journal (Variables|/Script/DES502_Build.DES_JournalManager|GetJournal _journalmanager))
  (bind _chronology (Variables|/Script/DES502_Build.DES_JournalManager|GetChronology _journalmanager))
  (bind _entries (Utilities|Struct|BreakDES_JournalStruct _journal))
  ;[0.05098 0.05098 0.05098] CAPTURE POLAROID: Calculate the scores of visible curios...
  (bind _curiototalscores (CallFunction|GetCuriosinView))
  ;[0.05098 0.05098 0.05098] // DEBUG: Printing all registered scores...
  (bind _keys (Utilities|Map|Keys _curiototalscores))
  (for _array_element _keys
    _)
  ;[0.05127 0.05127 0.05127] ...Check which (if any) journal entry should be updated...
  (bind (_valid _validid) (CallFunction|GetValidCurio _curiototalscores))
  (if _valid
    ;[0.05098 0.05098 0.05098] ...Capture the scene in the appropriate RenderTarget...
    (bind _structout (Utilities|Struct|SetmembersinDES_JournalEntryStruct (.Value (Utilities|Map|Find _entries _validid)) (Utilities|Array|Length _chronology)))
    (Utilities|Map|Add _entries _validid _structout)
    (Utilities|Array|Add _chronology _validid)
    (Variables|/Script/Engine.SceneCaptureComponent2D|SetTextureTarget _scenecapturecomponent2d (.RenderTarget (Utilities|Struct|BreakDES_JournalEntryStruct _structout)))
    (Rendering|SceneCapture|CaptureScene _scenecapturecomponent2d :!class /Script/Engine.SceneCaptureComponent2D)
    (for _array_element_2 _chronology
      (Development|PrintString (Utilities|String|Append (Utilities|String|Append _array_element_2 ": ") (Utilities|String|ToString(Integer) (.EntryActive (Utilities|Struct|BreakDES_JournalEntryStruct (.Value (Utilities|Map|Find (Utilities|Struct|BreakDES_JournalStruct (Variables|/Script/DES502_Build.DES_JournalManager|GetJournal (Variables|/Script/DES502_Build.DESGameInstance|GetJournalManager (Variables|Default|GetDES_GameInstance)))) _array_element_2))))))))))

(fn GetCuriosinView
  (bind _curioscores (LocalVariables|GetCurioScores))
  (bind _scenecapturecomponent2d (Variables|Default|GetSceneCaptureComponent2D))
  ;[0.05098 0.05098 0.05098] GET CURIOS IN VIEW: For each curio nearby...
  (for _array_element (Collision|GetOverlappingActors (Variables|Default|GetSphere) "/Script/DES502_Build.DESCurio" :!class /Script/Engine.PrimitiveComponent)
    ;[0.05098 0.05098 0.05098] ...Check if and (roughly) where each is in view... // NB: Might be some subtleties to this, but should be fine if the polaroid doen't have a bigger FOV than the player's?
    (if (Class|Actor|WasRecentlyRendered _array_element 0.2)
      (if (<= (Class|KismetMathLibrary|DegAcos (Math|Vector|DotProduct (Math|Vector|Normalize (- (Transformation|GetActorLocation _array_element) (Transformation|GetWorldLocation _scenecapturecomponent2d))) (Math|Vector|GetForwardVector _scenecapturecomponent2d))) (* (Variables|/Script/Engine.SceneCaptureComponent2D|GetFOVAngle _scenecapturecomponent2d) (/ 9e+02 1.92e+03)))
        ;[0.05098 0.05098 0.05098] ...Initialise curio score (if appropriate)...
        (bind _asdescurio (Utilities|Casting|CastToDESCurio _array_element))
        (if (Utilities|Map|Contains (LocalVariables|GetCurioScores) (Variables|/Script/DES502_Build.DESCurio|GetID _asdescurio))
          _
          (else
            (Utilities|Map|Add (LocalVariables|GetCurioScores) (Variables|/Script/DES502_Build.DESCurio|GetID _asdescurio) 0.0)))
        ;[0.117 0.05127 0.117] ...Increase curio score... // FIXME: Currently an MVP, purely based on how many objects are on screen...
        (Utilities|Map|Add _curioscores (Variables|/Script/DES502_Build.DESCurio|GetID _asdescurio) (+ (.Value (Utilities|Map|Find _curioscores (Variables|/Script/DES502_Build.DESCurio|GetID _asdescurio))) 1.0)))))
  (return (LocalVariables|GetCurioScores)))

(fn GetValidCurio
  (params (CurioTotalScores :type Map%20of%20Strings%20to%20Reals))
  (bind _keys (Utilities|Map|Keys CurioTotalScores))
  (for _array_element _keys
    (if (.ReturnValue (Utilities|Map|Find (Utilities|Struct|BreakDES_JournalStruct (Variables|/Script/DES502_Build.DES_JournalManager|GetJournal (Variables|/Script/DES502_Build.DESGameInstance|GetJournalManager (Variables|Default|GetDES_GameInstance)))) _array_element))
      (if (< (.EntryActive (Utilities|Struct|BreakDES_JournalEntryStruct (.Value (Utilities|Map|Find (Utilities|Struct|BreakDES_JournalStruct (Variables|/Script/DES502_Build.DES_JournalManager|GetJournal (Variables|/Script/DES502_Build.DESGameInstance|GetJournalManager (Variables|Default|GetDES_GameInstance)))) _array_element)))) 0)
        (if (> (.Value (Utilities|Map|Find CurioTotalScores _array_element)) (LocalVariables|GetMaxValidScore))
          (LocalVariables|SetMaxValidScore (.Value (Utilities|Map|Find CurioTotalScores _array_element)))
          (LocalVariables|SetMaxValidID _array_element)))))
  (return (> (LocalVariables|GetMaxValidScore) 0.0) (LocalVariables|GetMaxValidID)))