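; Wisp cluster actor that repositions its wisp on a sphere-like offset around the cluster centre as the player approaches.
; Each Tick, it blends by horizontal player distance from a raised, camera-right offset when close to the side opposite the player when farther away.
; Camera yaw comes from the player camera manager to avoid hard references, and the clamped lerp sets the wisp's relative location.
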(event EventTick
  (params (DeltaSeconds :type Float%20%28single-precision%29))
  (bind _returnvalue (Game|GetPlayerCharacter 0))
  (bind _returnvalue_2 (Transformation|GetActorLocation))
  (bind _returnvalue_3 (Transformation|GetActorLocation _returnvalue))
  (bind _returnvalue_4 (- _returnvalue_3 _returnvalue_2))
  (Transformation|SetRelativeLocation (Variables|Default|GetBP_Wisp) (Math|Vector|Lerp(Vector) (* (Variables|Default|GetRadius) (Math|Vector|RotateVector (Class|KismetMathLibrary|VectorForward) (Math|Rotator|MakeRotator 0.0 45.0 (+ (.yaw (Camera|GetCameraRotation (Game|GetPlayerCameraManager 0))) 9e+01)))) (* (* (Variables|Default|GetRadius) -1.0) (Math|Vector|Normalize (Math|Vector|MakeVector (.x _returnvalue_4) (.y _returnvalue_4) 0.0))) (Math|Float|Clamp(Float) (/ (Math|Vector|VectorLength (Math|Vector|MakeVector (.x _returnvalue_4) (.y _returnvalue_4) 0.0)) 2.5e+02) 0.0 1.0)) false false))

(fn ConstructionScript)