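; Crowbar actor that is both a world pickup and the player's swingable tool for breaking boards, with much of its logic still named "pickaxe".
; Unowned copies increment the inventory count on player overlap and self-destruct, with the first equipping the crowbar if scrolling is allowed.
; Shooting locks the inventory and fakes a swing with timelines on the shoulder pivot.
; A scale-adjusted HitSphere hits boards on overlap, with a mid-swing query as failsafe.
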(event OnComponentBeginOverlap(CollisionSphere)
  (params (OverlappedComponent :type Primitive%20Component%20Object%20Reference) (OtherActor :type Actor%20Object%20Reference) (OtherComp :type Primitive%20Component%20Object%20Reference) (OtherBodyIndex :type Integer) (bFromSweep :type Boolean) (SweepResult :type Hit%20Result%20Structure%20%28by%20ref%29))
  (bind _des_gameinstance (Variables|Default|GetDES_GameInstance))
  (bind _firstpersoncharacter (Variables|Default|GetFirstPersonCharacter))
  (bind _gamedata (Variables|/Script/DES502_Build.DESGameInstance|GetGameData _des_gameinstance))
  ;[0.05127 0.05127 0.05127] BEGIN OVERLAP: If not owned by the player, add to counter and destroy...
  (Utilities|Casting|CastToBP_FirstPersonCharacter OtherActor)
  (Utilities|Casting|CastToBP_FirstPersonCharacter (Components|GetOwner)
    (:CastFailed
      (bind _output_get (Variables|/Script/DES502_Build.DESSaveGame|SetCrowbarInventoried _gamedata (+ (Variables|/Script/DES502_Build.DESSaveGame|GetCrowbarInventoried _gamedata) 1)))
      (bind _scroll (Default|CanScrollInventory (Variables|Default|GetFirstPersonCharacter)))
      (if (and (== _output_get 1) _scroll)
        (Variables|/Script/DES502_Build.DESSaveGame|SetPlayerHandheld (Variables|/Script/DES502_Build.DESGameInstance|GetGameData (Variables|Default|GetDES_GameInstance)) "ECrowbar")
        (Default|ShowInventory _firstpersoncharacter)
        (Default|TutorialiseRaisePickaxe _firstpersoncharacter))
      (Actor|DestroyActor))))

(event OnComponentBeginOverlap(HitSphere)
  (params (OverlappedComponent :type Primitive%20Component%20Object%20Reference) (OtherActor :type Actor%20Object%20Reference) (OtherComp :type Primitive%20Component%20Object%20Reference) (OtherBodyIndex :type Integer) (bFromSweep :type Boolean) (SweepResult :type Hit%20Result%20Structure%20%28by%20ref%29))
  ;[0.05098 0.05098 0.05098] BEGIN OVERLAP: Deactivate the overlapping BP_Board, if it hasn't been already...
  (if (Variables|Default|GetPickaxeLocked)
    (bind _asbp_board (Utilities|Casting|CastToBP_Board OtherActor))
    (Default|OnPickaxed _asbp_board (Transformation|GetWorldLocation (Variables|Default|GetHitSphere)))))

(event Input|EnhancedActionEvents|EnhancedInputActionIA_Shoot
  (params (ActionValue :type Boolean) (ElapsedSeconds :type Float%20%28double-precision%29) (TriggeredSeconds :type Float%20%28double-precision%29) (InputAction :type Input%20Action%20Object%20Reference :default "/Game/Prefabs/FirstPerson/Input/Actions/IA_Shoot.IA_Shoot"))
  (bind _firstpersoncharacter (Variables|Default|GetFirstPersonCharacter))
  (bind _des_gameinstance (Variables|Default|GetDES_GameInstance))
  (bind _des_gameinstance_2 (Variables|Default|GetDES_GameInstance))
  (bind _gamedata (Variables|/Script/DES502_Build.DESGameInstance|GetGameData _des_gameinstance_2))
  (bind _shoulderpivot (Variables|/Game/Blueprints/BP_FirstPersonCharacter.BP_FirstPersonCharacter_C|GetShoulderPivot _firstpersoncharacter))
  ;[0.05098 0.05098 0.05098] IA SHOOT: If possible...
  (:Triggered
    (if (and (Variables|/Script/DES502_Build.DESGameInstance|GetPlayerHandheldActive _des_gameinstance) (Math|Boolean|NORBoolean (Variables|/Script/DES502_Build.DESGameInstance|GetPickaxeSwung _des_gameinstance) (Variables|Default|GetPickaxeLocked)))
      ;[0.05098 0.05098 0.05098] ...Lock the inventory while the swing plays...
      (Variables|/Script/DES502_Build.DESGameInstance|SetPickaxeSwung _des_gameinstance_2 true)
      (Variables|Default|SetPickaxeLocked true)
      (Variables|/Script/DES502_Build.DESSaveGame|SetTutorialisedRaisePickaxe _gamedata true)
      (Variables|/Script/DES502_Build.DESSaveGame|SetTutorialisedSwingPickaxe _gamedata true)
      ;[0.117 0.05127 0.117] ...Manually swing pickaxe... // NB: A very hacky action, due to lack of skeletal animation...
      (Variables|Default|SetShoulderRotation (Variables|/Script/Engine.SceneComponent|GetRelativeRotation _shoulderpivot))
      (Variables|Default|SetShoulderLocation (Variables|/Script/Engine.SceneComponent|GetRelativeLocation _shoulderpivot))
      (Components|Timeline|SetPlayRate (Variables|Default|GetSwingForwardTimeline) (/ 1.0 0.1836))
      (bind _swing (Timeline|SwingForwardTimeline PlayFromStart)
        (:Update
          (Transformation|SetRelativeRotation (Variables|/Game/Blueprints/BP_FirstPersonCharacter.BP_FirstPersonCharacter_C|GetShoulderPivot (Variables|Default|GetFirstPersonCharacter)) (Math|Rotator|CombineRotators (Variables|Default|GetShoulderRotation) (* "-60.000000,0.000000,0.000000" _swing)) false false)
          (Transformation|SetRelativeLocation (Variables|/Game/Blueprints/BP_FirstPersonCharacter.BP_FirstPersonCharacter_C|GetShoulderPivot (Variables|Default|GetFirstPersonCharacter)) (+ (Variables|Default|GetShoulderLocation) (* "-2.000000,0.000000,27.000000" _swing)) false false))
        (:Finished
          (CallFunction|HitNearbyBoards)
          (Audio|PlaySound2D "/Game/Audio/Assets/SwingPickaxe.SwingPickaxe" 1.0 1.0 0.0 0 0)
          (Components|Timeline|SetPlayRate (Variables|Default|GetSwingBackwardTimeline) (/ 1.0 0.15))
          (bind _newtrack_0 (Timeline|SwingBackwardTimeline PlayFromStart)
            (:Update
              (Transformation|SetRelativeRotation (Variables|/Game/Blueprints/BP_FirstPersonCharacter.BP_FirstPersonCharacter_C|GetShoulderPivot (Variables|Default|GetFirstPersonCharacter)) (Math|Rotator|CombineRotators (Variables|Default|GetShoulderRotation) (* "-60.000000,0.000000,0.000000" _newtrack_0)) false false)
              (Transformation|SetRelativeLocation (Variables|/Game/Blueprints/BP_FirstPersonCharacter.BP_FirstPersonCharacter_C|GetShoulderPivot (Variables|Default|GetFirstPersonCharacter)) (+ (Variables|Default|GetShoulderLocation) (* "-2.000000,0.000000,27.000000" _newtrack_0)) false false))
            (:Finished
              ;[0.05098 0.05098 0.05098] ...Unlock the inventory...
              (Variables|/Script/DES502_Build.DESGameInstance|SetPickaxeSwung (Variables|Default|GetDES_GameInstance) false)
              (Variables|Default|SetPickaxeLocked false)
              ;[0.05098 0.05098 0.05098] BUGFIX: If the iron sights have been released since the pickaxe animation started, then lower them...
              (if (not (Input|EnhancedActionValues|GetIA_Zoomed))
                (Default|DelayedIAZoomOut (Variables|Default|GetFirstPersonCharacter))))))))))

(event EventBeginPlay
  (bind _hitsphere (Variables|Default|GetHitSphere))
  ;[0.05098 0.05098 0.05098] BEGIN PLAY: Adjust hitboxes to camera trickery...
  (|CallParentFunction)
  (Components|Sphere|SetSphereRadius _hitsphere (/ (Variables|/Script/Engine.SphereComponent|GetSphereRadius _hitsphere) (.x (Variables|/Script/Engine.SceneComponent|GetRelativeScale3D (Variables|/Game/Blueprints/BP_FirstPersonCharacter.BP_FirstPersonCharacter_C|GetArmMesh (Variables|Default|GetFirstPersonCharacter))))) true))

(fn ConstructionScript
  (|CallParentFunction))

(fn HitNearbyBoards
  ;[0.05098 0.05098 0.05098] HIT NEARBY BOARDS: Deactivate all BP_Boards in range... // NB: Included at midpoint of the swing as a failsafe for collision detection...
  (for _array_element (Collision|GetOverlappingActors (Variables|Default|GetHitSphere) "/Game/Blueprints/BP_Board.BP_Board_C" :!class /Script/Engine.PrimitiveComponent)
    (bind _asbp_board (Utilities|Casting|CastToBP_Board _array_element))
    (Default|OnPickaxed _asbp_board (Transformation|GetWorldLocation (Variables|Default|GetHitSphere)))))