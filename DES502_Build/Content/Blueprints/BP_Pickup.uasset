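; BP_Pickup is a pickup actor that can be activated as a player handheld, possibly a Polaroid going by a FIXME.
; On BeginPlay it caches the game instance and first-person character.
; An overlap on its collision sphere destroys it unless that character owns it.
; ActivateHandheld stores the given player, enables input and adds the IMC_Weapons Enhanced Input mapping context, marked as a placeholder for IMC_Polaroid.
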(event OnComponentBeginOverlap(CollisionSphere)
  (params (OverlappedComponent :type Primitive%20Component%20Object%20Reference) (OtherActor :type Actor%20Object%20Reference) (OtherComp :type Primitive%20Component%20Object%20Reference) (OtherBodyIndex :type Integer) (bFromSweep :type Boolean) (SweepResult :type Hit%20Result%20Structure%20%28by%20ref%29))
  ;[0.05127 0.05127 0.05127] BEGIN OVERLAP: If not owned by the player, destroy...
  (Utilities|Casting|CastToBP_FirstPersonCharacter (Components|GetOwner)
    (:CastFailed
      (Actor|DestroyActor))))

(event EventBeginPlay
  ;[0.05127 0.05127 0.05127] BEGIN PLAY: Create reference to DES_GameInstance...
  (bind _asdesgame_instance (Utilities|Casting|CastToDESGameInstance (Game|GetGameInstance)))
  (Variables|Default|SetDES_GameInstance _asdesgame_instance)
  (bind _asbp_first_person_character (Utilities|Casting|CastToBP_FirstPersonCharacter (Game|GetPlayerCharacter 0)))
  (Variables|Default|SetFirstPersonCharacter _asbp_first_person_character))

(fn ConstructionScript)

(fn ActivateHandheld
  (params (Player :type BP%20First%20Person%20Character%20Object%20Reference))
  ;[0.2159 0.05127 0.05127] SWITCH TO HANDHELD: Attach IMC_Weapons mapping context... // FIXME: Create IMC_Polaroid mapping context... // FIXME: Can delete the 'Set Player' step?
  (Variables|Default|SetFirstPersonCharacter Player)
  (bind _asplayer_controller (Utilities|Casting|CastToPlayerController (Pawn|GetController Player)))
  (Input|EnableInput _asplayer_controller)
  (Utilities|IsValid (PlayerController|LocalPlayerSubsystems|GetEnhancedInputLocalPlayerSubsystem _asplayer_controller)
    (:Is%20Valid
      (Input|AddMappingContext (PlayerController|LocalPlayerSubsystems|GetEnhancedInputLocalPlayerSubsystem _asplayer_controller) "/Game/Prefabs/FirstPerson/Input/IMC_Weapons.IMC_Weapons" 0 "(bIgnoreAllPressedKeysUntilRelease=True,bForceImmediately=False)"))))