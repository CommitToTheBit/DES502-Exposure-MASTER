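; BP_Boards is an actor with three attached boards that the player knocks loose with a crowbar.
; BeginPlay caches the game instance and character, fills the board array and adds the weapons input context.
; While the crowbar is handheld, each shoot trigger detaches the next board, enabling physics and pushing it toward the player.
; Proximity-based crowbar switching is deactivated, so detaching has no range check and can hit multiple instances at once.
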(event OnComponentBeginOverlap(CollisionSphere)
  (params (OverlappedComponent :type Primitive%20Component%20Object%20Reference) (OtherActor :type Actor%20Object%20Reference) (OtherComp :type Primitive%20Component%20Object%20Reference) (OtherBodyIndex :type Integer) (bFromSweep :type Boolean) (SweepResult :type Hit%20Result%20Structure%20%28by%20ref%29))
  ;[0.2159 0.05127 0.05127] BEGIN OVERLAP: If possible, raise crowbar... // FIXME: Deactivated due to inventory restructure!
  (if (== OtherActor (Variables|Default|GetFirstPersonCharacter))
    _))

(event OnComponentEndOverlap(CollisionSphere)
  (params (OverlappedComponent :type Primitive%20Component%20Object%20Reference) (OtherActor :type Actor%20Object%20Reference) (OtherComp :type Primitive%20Component%20Object%20Reference) (OtherBodyIndex :type Integer))
  ;[0.2159 0.05127 0.05127] END OVERLAP: If possible, lower crowbar... // FIXME: Deactivated due to inventory restructure!
  (if (== OtherActor (Variables|Default|GetFirstPersonCharacter))
    _))

(event Input|EnhancedActionEvents|EnhancedInputActionIA_Shoot
  (params (ActionValue :type Boolean) (ElapsedSeconds :type Float%20%28double-precision%29) (TriggeredSeconds :type Float%20%28double-precision%29) (InputAction :type Input%20Action%20Object%20Reference :default "/Game/Prefabs/FirstPerson/Input/Actions/IA_Shoot.IA_Shoot"))
  (bind _boardsattached (Variables|Default|GetBoardsAttached))
  ;[0.2159 0.05127 0.05127] IA_SHOOT: If possible, use a handheld crowbar to detach a remaining board... // FIXME: Assumes crowbar applies to multiple BP_Board instances at once!
  (:Triggered
    (if (and (Utilities|Enum|Equal(Enum) (Variables|/Script/DES502_Build.DESSaveGame|GetPlayerHandheld (Variables|/Script/DES502_Build.DESGameInstance|GetGameData (Variables|Default|GetDES%20Game%20Instance))) "ECrowbar") (> (Utilities|Array|Length (Variables|Default|GetBoardsAttached)) 0))
      (CallFunction|DetachBoard (Utilities|Array|Get(acopy) _boardsattached))
      (Utilities|Array|RemoveIndex _boardsattached))))

(event EventBeginPlay
  (bind _returnvalue (Game|GetPlayerController 0))
  (bind _returnvalue_2 (PlayerController|LocalPlayerSubsystems|GetEnhancedInputLocalPlayerSubsystem _returnvalue))
  ;[0.05127 0.05127 0.05127] BEGIN PLAY: Create reference to DES_GameInstance...
  (bind _asdesgame_instance (Utilities|Casting|CastToDESGameInstance (Game|GetGameInstance)))
  (Variables|Default|SetDES%20Game%20Instance _asdesgame_instance)
  ;[0.05098 0.05098 0.05098] ...Create reference to player character...
  (bind _asbp_first_person_character (Utilities|Casting|CastToBP_FirstPersonCharacter (Game|GetPlayerCharacter 0)))
  (Variables|Default|SetFirstPersonCharacter _asbp_first_person_character)
  ;[0.05098 0.05098 0.05098] ...Initialise array of attached boards...
  (Utilities|Array|Add (Variables|Default|GetBoardsAttached) (Variables|Default|GetBoard1))
  (Utilities|Array|Add (Variables|Default|GetBoardsAttached) (Variables|Default|GetBoard2))
  (Utilities|Array|Add (Variables|Default|GetBoardsAttached) (Variables|Default|GetBoard3))
  ;[0.2159 0.05127 0.05127] SWITCH TO HANDHELD: Attach IMC_Weapons mapping context... // FIXME: Create IMC_Polaroid mapping context...
  (Input|EnableInput _returnvalue)
  (Utilities|IsValid _returnvalue_2
    (:Is%20Valid
      (Input|AddMappingContext _returnvalue_2 "/Game/Prefabs/FirstPerson/Input/IMC_Weapons.IMC_Weapons" 0 "(bIgnoreAllPressedKeysUntilRelease=True,bForceImmediately=False)"))))

(fn ConstructionScript)

(fn DetachBoard
  (params (Board :type Static%20Mesh%20Component%20Object%20Reference))
  ;[0.05098 0.05098 0.05098] DETACH BOARD: Enable physics...
  (Physics|SetSimulatePhysics Board true)
  ;[0.117 0.05127 0.117] ...Knock board forward in the direction of the player... // FIXME: Most basic implementation possible!
  (Physics|AddImpulse Board (* (Math|Vector|Normalize (- (Transformation|GetActorLocation (Variables|Default|GetFirstPersonCharacter)) (Transformation|GetWorldLocation Board))) 1e+02) "None" true))