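; BP_VignetteTrigger is an actor with inner and outer spheres; despite its name, it contains no overlap or vignette logic.
; On BeginPlay it stores each sphere's local bounds size times world scale as OuterRadii and InnerRadii, which are full extents rather than half-extents.
; It prints both values and the inner sphere's world rotation for debugging.
; A disconnected node chain would negate that rotation but never runs.
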(event EventBeginPlay
  (bind _innersphere (Variables|Default|GetInnerSphere))
  (bind _outersphere (Variables|Default|GetOuterSphere))
  (bind (_min _max) (Components|StaticMesh|GetLocalBounds _innersphere))
  (bind (_min_2 _max_2) (Components|StaticMesh|GetLocalBounds _outersphere))
  (Variables|Default|SetOuterRadii (* (- _max_2 _min_2) (Transformation|GetWorldScale _outersphere)))
  (Variables|Default|SetInnerRadii (* (- _max _min) (Transformation|GetWorldScale _innersphere)))
  (Development|PrintString (Utilities|String|ToString(Vector) (Variables|Default|GetOuterRadii)))
  (Development|PrintString (Utilities|String|ToString(Vector) (Variables|Default|GetInnerRadii)))
  (Development|PrintString (Utilities|String|ToString(Rotator) (Transformation|GetWorldRotation (Variables|Default|GetInnerSphere)))))

(fn ConstructionScript)