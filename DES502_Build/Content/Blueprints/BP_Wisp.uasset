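; BP_Wisp is a wisp actor with a non-colliding mesh that constantly turns to face the player character.
; BeginPlay disables collision on the mesh.
; Every Tick, it takes the normalized direction to player 0's character, converts it to pitch and yaw, and sets the actor rotation directly with zero roll and no interpolation.
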(event EventBeginPlay
  (Collision|SetCollisionEnabled (Variables|Default|GetMesh) "NoCollision"))

(event EventTick
  (params (DeltaSeconds :type Float%20%28single-precision%29))
  (bind _returnvalue (Game|GetPlayerCharacter 0))
  (bind _returnvalue_2 (Transformation|GetActorLocation))
  (bind _returnvalue_3 (Transformation|GetActorLocation _returnvalue))
  (bind _returnvalue_4 (- _returnvalue_3 _returnvalue_2))
  (bind _returnvalue_5 (Math|Vector|Normalize _returnvalue_4))
  (bind (_yaw _pitch) (Math|Vector|GetYawPitchfromVector _returnvalue_5))
  (Transformation|SetActorRotation (Math|Rotator|MakeRotator 0.0 _pitch _yaw)))

(fn ConstructionScript)