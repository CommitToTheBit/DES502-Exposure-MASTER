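; BP_Board is a board that the player knocks loose with a pickaxe.
; On the first OnPickaxed event it enables physics, ignores Pawn collision and gets pushed away from the hit origin.
; X/Y tumble is pseudo-random, from a sine of the hit direction's dot with the up vector.
; Z spin follows the signed square of the forward dot, mirrored by hit side; accurate physics and item destruction remain a FIXME.
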(event Custom|OnPickaxed
  (params (Origin :type Vector))
  (bind _boardmesh (Variables|Default|GetBoardMesh))
  ;[0.05098 0.05098 0.05098] ON PICKAXED: Ignore the player walking over the board...
  (if (not (Variables|Default|GetPickaxed))
    (Variables|Default|SetPickaxed true)
    (Physics|SetSimulatePhysics _boardmesh true)
    (Collision|SetCollisionResponsetoChannel _boardmesh "ECC_Pawn" "ECR_Ignore")
    ;[0.117 0.05127 0.117] ...Knock board away from the player... // FIXME: A full implementation would have more accurate physics, and item destruction...
    (bind _output_get (Variables|Default|SetPickaxeVector (Math|Vector|Normalize (- (Transformation|GetActorLocation) Origin))))
    (Physics|AddImpulse (Variables|Default|GetBoardMesh) (* _output_get 3e+02) "None" true)
    ;[0.05098 0.05098 0.05098] ...Add a (random) impulse about the x-, y-axes...
    (Class|PrimitiveComponent|AddAngularImpulseinDegrees (Variables|Default|GetBoardMesh) (Math|Vector|MakeVector (* (Math|Trig|Sin(Degrees) (* (Math|Vector|DotProduct (Variables|Default|GetPickaxeVector) (Math|Vector|GetUpVector (Variables|Default|GetBoardMesh))) 1e+03)) 1.5e+02) (* (Math|Trig|Sin(Degrees) (* (Math|Vector|DotProduct (Variables|Default|GetPickaxeVector) (Math|Vector|GetUpVector (Variables|Default|GetBoardMesh))) 1e+03)) 1.5e+02) 0.0) "None" true)
    ;[0.05098 0.05098 0.05098] ...Apply a (true) angular impulse about the z-axis..
    (if (>= (Math|Vector|DotProduct (Variables|Default|GetPickaxeVector) (Math|Vector|GetRightVector (Variables|Default|GetBoardMesh))) 0.0)
      (Variables|Default|SetPickaxeVector (- "" (Variables|Default|GetPickaxeVector))))
    (Class|PrimitiveComponent|AddAngularImpulseinDegrees (Variables|Default|GetBoardMesh) (Math|Vector|MakeVector 0.0 0.0 (* (* (Math|Float|Sign(Float) (Math|Vector|DotProduct (Variables|Default|GetPickaxeVector) (Math|Vector|GetForwardVector (Variables|Default|GetBoardMesh)))) (Math|Float|Square (Math|Vector|DotProduct (Variables|Default|GetPickaxeVector) (Math|Vector|GetForwardVector (Variables|Default|GetBoardMesh))))) 3e+02)) "None" true)))

(fn ConstructionScript)